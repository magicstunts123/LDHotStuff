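; Game instance for the Ant game that owns persistent save data, audio volume setup and achievement unlocking.
; On Init it loads the "Ant" save slot, or creates and saves a new one, then applies the saved master, music and SFX volumes through sound mix class overrides.
; Achievement unlocks are recorded on the save object and immediately written back to the slot.
; A menu level-open node is present but unconnected.
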(event `self.ReceiveInit`
  (bind _returnvalue (`GameplayStatics.DoesSaveGameExist` "Ant"))
  (if _returnvalue
    (bind _returnvalue_2 (`GameplayStatics.LoadGameFromSlot` "Ant"))
    (bind _asbp_ant_save (cast `/Game/WB_Thomas/BP_AntSave` _returnvalue_2))
    (set `self.As BP Ant Save` _asbp_ant_save)
    (`KismetSystemLibrary.PrintString` "Loaded Save")
    (`self.SetVolumes`)
    (else
      (bind _returnvalue_3 (`GameplayStatics.CreateSaveGameObject` "/Game/WB_Thomas/BP_AntSave.BP_AntSave_C"))
      (bind _output_get (set `self.As BP Ant Save` _returnvalue_3))
      (`GameplayStatics.SaveGameToSlot` _output_get "Ant")
      (`KismetSystemLibrary.PrintString` "Created New Save")
      (`self.SetVolumes`)))
  (`KismetSystemLibrary.Delay` 0.2))

(event `UnlockAchievement`
  (params (Achievement :type "/Game/WB_Thomas/E_Achievements Enum" :default "NewEnumerator0"))
  (`/Game/WB_Thomas/BP_AntSave.UnlockAchievement` (`self.As BP Ant Save`) Achievement)
  (`self.SaveAntGame`))

(event `SaveAntGame`
  (bind _returnvalue (`GameplayStatics.SaveGameToSlot` (`self.As BP Ant Save`) "Ant"))
  (if _returnvalue
    (`KismetSystemLibrary.PrintString` "Saved Game")))

(fn `SetVolumes`
  (bind (_volumesets_master _volumesets_music _volumesets_sfx) (break `/Game/WB_Thomas/F_VolumeSettings` (`/Game/WB_Thomas/BP_AntSave.VolumeSets` (`self.As BP Ant Save`))))
  (`GameplayStatics.SetSoundMixClassOverride` "/Game/Audio/MainMix.MainMix" "/Game/Audio/AudioMainClass.AudioMainClass" _volumesets_master 1.0 0.0)
  (`GameplayStatics.SetSoundMixClassOverride` "/Game/Audio/MainMix.MainMix" "/Game/Audio/MusicSoundClass.MusicSoundClass" _volumesets_music 1.0 0.0)
  (`GameplayStatics.SetSoundMixClassOverride` "/Game/Audio/MainMix.MainMix" "/Game/Audio/SFXSoundClass.SFXSoundClass" _volumesets_sfx 1.0 0.0)
  (`GameplayStatics.PushSoundMixModifier` "/Game/Audio/MainMix.MainMix"))