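; Inventory component that tracks how many of each item its owner holds.
; Items is a map from item ID to quantity, where adding increments an existing stack or creates one at 1.
; Removing decrements the stack and returns whether the ID was found, without deleting the entry or stopping at zero.
; Helper functions expose the existence check, per-item quantity and whole map, with no event-driven logic.
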(fn `AddItemToInventory`
  (params (Item_ID :type Name))
  (if (`self.ItemTypeAlreadyExist?` (`local.Item_ID`))
    ;[1 1 1] Added 1 zu bestehenden Stack
    (`BlueprintMapLibrary.Map_Add` (`self.Items`) (`local.Item_ID`) (+ (`self.GetItemQty` (`local.Item_ID`)) 1))
    (else
      ;[1 1 1] ErstelltStack
      (`BlueprintMapLibrary.Map_Add` (`self.Items`) (`local.Item_ID`) 1))))

(fn `GetItemQty`
  (params (ItemID :type Name))
  (returns (Quantity :type Integer))
  (return (`BlueprintMapLibrary.Map_Find` (`self.Items`) ItemID)))

(fn `GetItems`
  (returns (Items :type "Map of Name to Integer"))
  (return (`self.Items`)))

(fn `ItemTypeAlreadyExist?`
  (params (Key :type "Name (by ref)"))
  (returns (ReturnValue :type Boolean) (Value :type Integer))
  (bind (_value _returnvalue) (`BlueprintMapLibrary.Map_Find` (`self.Items`) Key))
  (return _returnvalue _value))

(fn `RemoveFromInventory`
  (params (ItemID :type Name))
  (returns (Success :type Boolean))
  (bind (_returnvalue _value) (`self.ItemTypeAlreadyExist?` ItemID))
  (if _returnvalue
    (`BlueprintMapLibrary.Map_Add` (`self.Items`) (`local.ItemID`) (- _value 1))
    (return true)
    (else
      (return false))))