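; BP_Gluehwuermchen is a firefly actor that follows the player pawn, hovering above it.
; A looping timer picks a new random horizontal offset around the player every few seconds.
; Tick eases the actor toward that offset point with a swept VInterpTo move and turns it to face that point.
; A timeline started at BeginPlay drives the mesh's relative height to add vertical motion on top of the follow movement.
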(event `self.ReceiveBeginPlay`
  (`KismetSystemLibrary.K2_SetTimerDelegate` (delegate `ChangeTargetLoc`) 3.0 true)
  (bind (_direction _alpha) (`Timeline|Timeline`)
    (:`Update`
      (`SceneComponent.K2_SetRelativeLocation` (`self.StaticMesh`) (`KismetMathLibrary.MakeVector` 0.0 0.0 (`KismetMathLibrary.Lerp` 0.0 30.0 _alpha)) false false))))

(event `ChangeTargetLoc`
  (bind _returnvalue (`KismetMathLibrary.RandomFloatInRange` -60.0 60.0))
  (set `self.Y` _returnvalue)
  (set `self.X` _returnvalue))

(event `self.ReceiveTick`
  (params (DeltaSeconds :type "Float (single-precision)"))
  (bind _returnvalue (`self.K2_GetActorLocation`))
  (bind _returnvalue_2 (+ (`self.K2_GetActorLocation` (`GameplayStatics.GetPlayerPawn` 0)) (`KismetMathLibrary.MakeVector` (`self.X`) (`self.Y`) 160.0)))
  (`self.K2_SetActorLocation` (`KismetMathLibrary.VInterpTo` _returnvalue _returnvalue_2 DeltaSeconds 8.0) true)
  (`self.K2_SetActorRotation` (`KismetMathLibrary.FindLookAtRotation` _returnvalue _returnvalue_2)))

(fn `UserConstructionScript`)