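; BP_AntSave is a save data Blueprint that holds the game's achievement states and volume settings.
; UnlockAchievement switches on the given achievement and calls UnlockElement, currently only with index 0, to mark that entry in the Achievements array as unlocked.
; GetVolume and SetVolume read and write the Master, Music and SFX levels in a volume settings struct.
; These functions only change the stored variables and do not write to disk.
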(fn `GetVolume`
  (returns (VolumeStruct :type "/Game/WB_Thomas/F_VolumeSettings Structure"))
  (return (`self.VolumeSets`)))

(fn `SetVolume`
  (params (Master :type "Float (double-precision)") (Music :type "Float (double-precision)") (SFX :type "Float (double-precision)"))
  (bind _volumesets (`self.VolumeSets`))
  (setmembers `/Game/WB_Thomas/F_VolumeSettings` :`StructRef` _volumesets :`Master` Master)
  (setmembers `/Game/WB_Thomas/F_VolumeSettings` :`StructRef` _volumesets :`Music` Music)
  (setmembers `/Game/WB_Thomas/F_VolumeSettings` :`StructRef` _volumesets :`SFX` SFX))

(fn `UnlockAchievement`
  (params (Achievement :type "/Game/WB_Thomas/E_Achievements Enum" :default "NewEnumerator0"))
  (switch `/Game/WB_Thomas/E_Achievements` Achievement
    (:`NewEnumerator0`
      (`self.UnlockElement` 0))))

(fn `UnlockElement`
  (params (AchievementIndex :type Integer))
  (setmembers `/Game/WB_Thomas/F_AchievementStruct` :`StructRef` (`|GetArrayItem` (`self.Achievements`) AchievementIndex) :`Unlocked` true))