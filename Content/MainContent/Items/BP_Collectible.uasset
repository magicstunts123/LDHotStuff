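; BP_Collectible is a pickup item that spins slowly and flies to the player when they come near.
; Entering the Sphere sets a follow flag and turns off physics on the Box, then Tick interpolates the actor toward the player pawn each frame.
; Overlapping the StaticMesh sends the ItemID to the player through an AddToInventory message and destroys the actor.
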(event `self.ReceiveTick`
  (params (DeltaSeconds :type "Float (single-precision)"))
  (`SceneComponent.K2_AddLocalRotation` (`self.StaticMesh`) (`KismetMathLibrary.MakeRotator` 0.0 0.0 (* DeltaSeconds 20.0)) false false)
  (if (`self.ShouldMoveToPlayer`)
    (bind (_sweephitresult _returnvalue) (`self.K2_SetActorLocation` (`KismetMathLibrary.VInterpTo` (`self.K2_GetActorLocation`) (`self.K2_GetActorLocation` (`GameplayStatics.GetPlayerPawn` 0)) (`GameplayStatics.GetWorldDeltaSeconds`) 5.0)))
    (if _returnvalue
      _)))

(event `self.Sphere.OnComponentBeginOverlap`
  (params (OverlappedComponent :type "PrimitiveComponent Object Reference") (OtherActor :type "Actor Object Reference") (OtherComp :type "PrimitiveComponent Object Reference") (OtherBodyIndex :type Integer) (bFromSweep :type Boolean) (SweepResult :type "HitResult Structure (by ref)"))
  (if (== OtherActor (`GameplayStatics.GetPlayerPawn` 0))
    (set `self.ShouldMoveToPlayer` true)
    (`PrimitiveComponent.SetSimulatePhysics` (`self.Box`) false)))

(event `self.StaticMesh.OnComponentBeginOverlap`
  (params (OverlappedComponent :type "PrimitiveComponent Object Reference") (OtherActor :type "Actor Object Reference") (OtherComp :type "PrimitiveComponent Object Reference") (OtherBodyIndex :type Integer) (bFromSweep :type Boolean) (SweepResult :type "HitResult Structure (by ref)"))
  (if (== OtherActor (`GameplayStatics.GetPlayerPawn` 0))
    (message `/Game/WB_Thomas/BPI_Interaction.AddToInventory` (`GameplayStatics.GetPlayerPawn` 0) (`self.ItemID`))
    (`self.K2_DestroyActor`)))

(fn `UserConstructionScript`)