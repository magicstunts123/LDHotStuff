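; BP_BrownSemen is a harvestable pickup that gives its item to the interacting actor and regrows afterwards.
; Interacting while IsReif (ripe) sends ItemID through AddToInventoryMessage, hides the mesh and disables the interaction sphere's collision.
; A two-minute timer fires Respawn, which restores visibility, query collision and the ripe flag.
; The money and item-check functions are empty stubs returning default values.
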(event `self.InteractWith`
  (params (InteractingActor :type "Actor Object Reference"))
  (if (`self.IsReif`)
    (message `/Game/WB_Thomas/BPI_Interaction.AddToInventory` InteractingActor (`self.ItemID`))
    (`SceneComponent.SetVisibility` (`self.StaticMeshComponent0`) false false)
    (`PrimitiveComponent.SetCollisionEnabled` (`self.InteractionSphere`) "NoCollision")
    (`KismetSystemLibrary.K2_SetTimerDelegate` (delegate `Respawn`) 120.0)
    (set `self.IsReif` false)))

(event `Respawn`
  (`SceneComponent.SetVisibility` (`self.StaticMeshComponent0`) true false)
  (`PrimitiveComponent.SetCollisionEnabled` (`self.InteractionSphere`) "QueryOnly")
  (set `self.IsReif` true))

(fn `AddMoney`
  (params (MoneyAdded :type Integer))
  (returns (NewMoney :type Integer))
  (return 0))

(fn `GetHasEnoughItems`
  (params (Item :type Name) (Qty :type Integer))
  (returns (HasEnough :type Boolean))
  (return false))

(fn `RemoveMoney`
  (params (MoneyToRemove :type Integer))
  (returns (Success :type Boolean) (NewMoney :type Integer))
  (return false 0))

(fn `UserConstructionScript`)