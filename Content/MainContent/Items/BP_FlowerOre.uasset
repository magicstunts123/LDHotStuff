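; BP_FlowerOre is an interactable item source that throws out a random item each time it is used.
; Every tick its Scene component yaws to face the player pawn.
; Interactwith spawns a random class from its Class array at the Arrow component, then launches the item's Box with a strong horizontal impulse along the arrow's forward direction.
; AddMoney, RemoveMoney and GetHasEnoughItems are stubs returning zero or false.
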(event `self.ReceiveTick`
  (params (DeltaSeconds :type "Float (single-precision)"))
  (bind (_returnvalue_roll _returnvalue_pitch _returnvalue_yaw) (`KismetMathLibrary.BreakRotator` (`KismetMathLibrary.FindLookAtRotation` (`self.K2_GetActorLocation`) (`self.K2_GetActorLocation` (`GameplayStatics.GetPlayerPawn` 0)))))
  (`SceneComponent.K2_SetWorldRotation` (`self.Scene`) (`KismetMathLibrary.MakeRotator` 0.0 0.0 _returnvalue_yaw) false false))

(event `self.InteractWith`
  (params (InteractingActor :type "Actor Object Reference"))
  (bind _arrow (`self.Arrow`))
  (bind (_returnvalue_x _returnvalue_y) (`KismetMathLibrary.BreakVector` (* (`KismetMathLibrary.Conv_RotatorToVector` (`SceneComponent.K2_GetComponentRotation` (`self.Arrow`))) 30000.0)))
  (bind _returnvalue (`|SpawnActorFromClass` (`KismetArrayLibrary.Array_Random` (`self.Class`)) (`KismetMathLibrary.MakeTransform` (+ (`SceneComponent.K2_GetComponentLocation` _arrow) (* (`SceneComponent.GetForwardVector` _arrow) (0.0 0.0 0.0)))) "AlwaysSpawn" "MultiplyWithRoot" null null))
  (`/Engine/EditorBlueprintResources/StandardMacros.IsValid` _returnvalue
    (:`Is Valid`
      (`PrimitiveComponent.AddImpulse` (`/Game/MainContent/Items/BP_Collectible.Box` _returnvalue) (`KismetMathLibrary.MakeVector` _returnvalue_x _returnvalue_y) "None" false))))

(fn `AddMoney`
  (params (MoneyAdded :type Integer))
  (returns (NewMoney :type Integer))
  (return 0))

(fn `GetHasEnoughItems`
  (params (Item :type Name) (Qty :type Integer))
  (returns (HasEnough :type Boolean))
  (return false))

(fn `RemoveMoney`
  (params (MoneyToRemove :type Integer))
  (returns (Success :type Boolean) (NewMoney :type Integer))
  (return false 0))

(fn `UserConstructionScript`)